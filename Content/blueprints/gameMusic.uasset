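; Game music actor that plays an audio component and exposes live left and right frequency spectrum arrays.
; BeginPlay sizes both arrays from NumExpectedParams and starts playback; the audio-finished event resets them to zeros.
; While music plays, Tick runs CalculateFrequencySpectrum on each channel over a short window at the current game time.
; GetRightParams and GetLeftParams return channel 1 and channel 2 results respectively.
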(event `self.MusicaGeneral.OnAudioFinished`
  (bind _output_get (set `self.exposedParam_r` (`|MakeArray` 0.0 :!type "Float (single-precision)") :!label _label))
  (for _ (range (+ (- (stale `EventBeginPlay` numExpectedParams) 2) 1))
    (`KismetArrayLibrary.Array_Add` _output_get)
    (set `self.exposedParam_l` (`self.exposedParam_r`))))

(event `EventBeginPlay`
  (params (numExpectedParams :type Integer))
  (`|ExecutionSequence`
    (:`then_0`
      (goto _label))
    (:`then_1`
      (`AudioComponent.Play` (`self.MusicaGeneral`) 0.0))))

(event `self.ReceiveTick`
  (params (DeltaSeconds :type "Float (single-precision)"))
  (if (`AudioComponent.IsPlaying` (`self.MusicaGeneral`))
    (for _index (range 1 3)
      (bind _outspectrum (`SoundVisualizationStatics.CalculateFrequencySpectrum` (`self.sound_wave`) _index (`GameplayStatics.GetTimeSeconds`) 0.1 (`KismetArrayLibrary.Array_Length` (`self.exposedParam_r`))))
      (switch `int` _index
        (:`1`
          (set `self.exposedParam_r` _outspectrum))
        (:`2`
          (set `self.exposedParam_l` _outspectrum))))))

(fn `GetLeftParams`
  (returns (LeftParams :type "Array of Float (double-precision)"))
  (return (`self.exposedParam_l`)))

(fn `GetRightParams`
  (returns (RightParams :type "Array of Float (double-precision)"))
  (return (`self.exposedParam_r`)))

(fn `UserConstructionScript`)