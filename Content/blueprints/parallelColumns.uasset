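; An actor holding two groups of column components, LeftColumns and RightColumns, whose individual lengths are set through a single function.
; ScaleColumn picks a side from a boolean, then scales each direct child on its X axis by the value at the same index in the supplied array, keeping Y and Z at one.
; The event graph and construction script are empty, so scaling happens only when ScaleColumn is called.
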(fn `Scale Column`
  (params (isLeft :type Boolean) (scaleVals :type "Array of Float (double-precision)"))
  (if isLeft
    (set `self.refChosenComp` (`self.leftColumns`))
    (else
      (set `self.refChosenComp` (`self.rightColumns`))))
  (for (_array_element _array_index) (`SceneComponent.GetChildrenComponents` (`self.refChosenComp`) false)
    (`SceneComponent.SetRelativeScale3D` _array_element (+ (* (`KismetMathLibrary.Vector_Forward`) (`|GetArrayItem` scaleVals _array_index)) (0.0 1.0 1.0)))))

(fn `UserConstructionScript`)